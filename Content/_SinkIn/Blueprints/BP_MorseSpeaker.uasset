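; Morse code speaker that signals a given code through particle bursts and short or long sounds.
; Play converts the code into an array of durations, which Tick steps through in a loop, toggling the particles on and off.
; Each switch-on plays the short sound if its duration equals the dot time, otherwise the long one.
; Stop halts the sequence and pauses the particles.
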(event EventBeginPlay
  (Niagara|ResetSystem (Variables|Default|GetParticles))
  (Class|NiagaraComponent|SetPaused (Variables|Default|GetParticles) true))

(event EventTick
  (params (DeltaSeconds :type Float%20%28single-precision%29))
  (if (Variables|Default|GetPlayParticles)
    (Variables|Default|SetCurrentTime (+ (Variables|Default|GetCurrentTime) DeltaSeconds))
    (if (>= (Variables|Default|GetCurrentTime) (Utilities|Array|Get(acopy) (Variables|Default|GetTimesArray) (Variables|Default|GetCurrentTimeIndex)))
      (Variables|Default|SetCurrentTime 0.0)
      (Variables|Default|SetCurrentTimeIndex (+ (Variables|Default|GetCurrentTimeIndex) 1))
      (if (>= (Variables|Default|GetCurrentTimeIndex) (Utilities|Array|Length (Variables|Default|GetTimesArray)))
        (Variables|Default|SetCurrentTimeIndex 0))
      (if (Variables|Default|GetParticlesActive)
        (Components|Activation|Deactivate (Variables|Default|GetParticles))
        (Variables|Default|SetParticlesActive false)
        (else
          (Components|Activation|SetActive (Variables|Default|GetParticles) true true)
          (Variables|Default|SetParticlesActive true)
          (bind _time1 (CallFunction|GetDotTime))
          (if (== (Utilities|Array|Get(acopy) (Variables|Default|GetTimesArray) (Variables|Default|GetCurrentTimeIndex)) _time1)
            (Audio|PlaySoundatLocation "/Game/_SinkIn/Sounds/Short__mp3cut_net_.Short__mp3cut_net_" (Transformation|GetWorldLocation (Variables|Default|GetParticles)) "0, 0, 0" 1.0 1.0 0.0 0 0 0 0)
            (else
              (Audio|PlaySoundatLocation "/Game/_SinkIn/Sounds/Long__mp3cut_net_.Long__mp3cut_net_" (Transformation|GetWorldLocation (Variables|Default|GetParticles)) "0, 0, 0" 1.0 1.0 0.0 0 0 0 0))))))))

(fn ConstructionScript)

(fn Play
  (params (MorseCode :type String))
  (bind _times (CallFunction|ConvertMorseCodetoTimeArray MorseCode))
  (Variables|Default|SetTimesArray _times)
  (Variables|Default|SetPlayParticles true)
  (Class|NiagaraComponent|SetPaused (Variables|Default|GetParticles) false)
  (Variables|Default|SetCurrentTimeIndex 0)
  (Variables|Default|SetCurrentTime 0.0)
  (Components|Activation|Deactivate (Variables|Default|GetParticles))
  (Variables|Default|SetParticlesActive false))

(fn Stop
  (Variables|Default|SetPlayParticles false)
  (Class|NiagaraComponent|SetPaused (Variables|Default|GetParticles) true))