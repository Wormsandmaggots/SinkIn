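; Treasure chest the player can carry on their back, drop via line trace, and unlock to win.
; On BeginPlay it shuffles tagged Morse cables and gives each a unique random color through dynamic materials.
; Interacting creates or toggles a lock widget showing those colors in cable order, with a password decoded from the cables' Morse codes, while restricting player actions.
; Opening the lock restores movement and shows the win screen.
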(event Custom|OnLockOpen_Event
  (params (Lock :type BP%20Treasure%20Lock%20Object%20Reference))
  (Widget|RemovefromParent Lock)
  (Variables|Default|SetLockVisible false)
  (Variables|/Script/Engine.PlayerController|SetbShowMouseCursor (Game|GetPlayerController 0) false)
  (Variables|/Game/ThirdPerson/Blueprints/BP_ThirdPersonCharacter.BP_ThirdPersonCharacter_C|SetCanInteractWithNotebook (stale EventInteract Player) true)
  (Variables|/Game/ThirdPerson/Blueprints/BP_ThirdPersonCharacter.BP_ThirdPersonCharacter_C|SetCanMove (stale EventInteract Player) true)
  (bind _returnvalue (UserInterface|CreateWidget "/Game/_SinkIn/Widgets/WBP_WinScreen.WBP_WinScreen_C"))
  (UserInterface|Viewport|AddtoViewport _returnvalue 10))

(event EventInteract
  (params (Player :type BP%20Third%20Person%20Character%20Object%20Reference))
  (Utilities|IsValid (Variables|Default|GetLock)
    (:Is%20Valid
      (if (Variables|Default|GetLockVisible)
        (Variables|/Game/ThirdPerson/Blueprints/BP_ThirdPersonCharacter.BP_ThirdPersonCharacter_C|SetCanPickup Player true)
        (Variables|/Game/ThirdPerson/Blueprints/BP_ThirdPersonCharacter.BP_ThirdPersonCharacter_C|SetCanInteractWithNotebook Player true)
        (Variables|/Game/ThirdPerson/Blueprints/BP_ThirdPersonCharacter.BP_ThirdPersonCharacter_C|SetCanMove Player true)
        (Widget|SetVisibility (Variables|Default|GetLock) "Collapsed")
        (Variables|Default|SetLockVisible false)
        (Variables|/Script/Engine.PlayerController|SetbShowMouseCursor (Game|GetPlayerController 0) false)
        (else
          (Variables|/Game/ThirdPerson/Blueprints/BP_ThirdPersonCharacter.BP_ThirdPersonCharacter_C|SetCanPickup Player false)
          (Variables|/Game/ThirdPerson/Blueprints/BP_ThirdPersonCharacter.BP_ThirdPersonCharacter_C|SetCanInteractWithNotebook Player false)
          (Variables|/Game/ThirdPerson/Blueprints/BP_ThirdPersonCharacter.BP_ThirdPersonCharacter_C|SetCanMove Player false)
          (Widget|SetVisibility (Variables|Default|GetLock) "Visible")
          (Variables|/Script/Engine.PlayerController|SetbShowMouseCursor (Game|GetPlayerController 0) true)
          (Variables|Default|SetLockVisible true)
          (Development|PrintString (CallFunction|GetCode)))))
    (:Is%20Not%20Valid
      (Variables|/Game/ThirdPerson/Blueprints/BP_ThirdPersonCharacter.BP_ThirdPersonCharacter_C|SetCanInteractWithNotebook Player false)
      (Variables|/Game/ThirdPerson/Blueprints/BP_ThirdPersonCharacter.BP_ThirdPersonCharacter_C|SetCanMove Player false)
      (bind _returnvalue (UserInterface|CreateWidget "/Game/_SinkIn/Widgets/BP_TreasureLock.BP_TreasureLock_C" (Game|GetPlayerController 0)))
      (Default|SetColors _returnvalue (Variables|Default|GetCoddingColors))
      (Variables|Default|SetLock _returnvalue)
      (EventDispatchers|AssignOnLockOpen _returnvalue (delegate Custom|OnLockOpen_Event))
      (Variables|/Game/_SinkIn/Widgets/BP_TreasureLock.BP_TreasureLock_C|SetPassword _returnvalue (CallFunction|GetCode))
      (UserInterface|Viewport|AddtoViewport _returnvalue 0)
      (Variables|/Script/Engine.PlayerController|SetbShowMouseCursor (Game|GetPlayerController 0) true)
      (Variables|Default|SetLockVisible true)
      (Variables|/Game/ThirdPerson/Blueprints/BP_ThirdPersonCharacter.BP_ThirdPersonCharacter_C|SetCanPickup Player false))))

(event EventBeginPlay
  (CallFunction|Init))

(event EventLeave
  (params (Player :type BP%20Third%20Person%20Character%20Object%20Reference))
  (Transformation|DetachFromActor "KeepWorld" "KeepWorld" "KeepWorld")
  (Collision|SetCollisionEnabled (Variables|Default|GetTreasure) "QueryOnly")
  (bind _outhit (Collision|LineTraceByChannel (Transformation|GetWorldLocation (Variables|Default|GetTreasure)) "0.000000,0.000000,-1000000.000000" "TraceTypeQuery1" false 0 "None"))
  (Transformation|SetWorldLocation (Variables|Default|GetDefaultSceneRoot) (Math|Vector|MakeVector (.X (Math|Vector|BreakVector (.Location (Collision|BreakHitResult _outhit)))) (.Y (Math|Vector|BreakVector (.Location (Collision|BreakHitResult _outhit)))) (+ (.Z (Math|Vector|BreakVector (.Location (Collision|BreakHitResult _outhit)))) 3e+01)) false false))

(event EventPickup
  (params (Player :type BP%20Third%20Person%20Character%20Object%20Reference))
  (Transformation|AttachActorToActor Player "BackHold" "SnapToTarget" "SnapToTarget" "KeepRelative" true)
  (Collision|SetCollisionEnabled (Variables|Default|GetTreasure) "NoCollision"))

(fn ConstructionScript)

(fn GetCode
  (for _array_element (Variables|Default|GetMorseCables)
    (bind _decrypted_value (CallFunction|GetNumberfromMorseCode (Variables|/Game/_SinkIn/Blueprints/BP_MorseCable.BP_MorseCable_C|GetRelatedMorseCode _array_element) (Variables|Default|GetMorseCodeDictionary)))
    (LocalVariables|SetNormalCode (Utilities|String|Append (LocalVariables|GetNormalCode) _decrypted_value)))
  (return (LocalVariables|GetNormalCode)))

(fn Init
  (bind _outactors (Actor|GetAllActorsOfClasswithTag "/Game/_SinkIn/Blueprints/BP_MorseCable.BP_MorseCable_C" (Variables|Default|GetCablesTag)))
  (bind _output_get (Variables|Default|SetMorseCables _outactors))
  (Utilities|Array|Shuffle _output_get)
  (for _array_element _output_get
    (bind _returnvalue (Rendering|Material|CreateDynamicMaterialInstance "/Game/_SinkIn/Materials/M_CableMaterial.M_CableMaterial" "None" "None" :!class /Script/Engine.KismetMaterialLibrary))
    (bind _output_get_2 (LocalVariables|SetPickedColor (.OutItem (Utilities|Array|Random (Variables|Default|GetDifferentColorMeshes)))))
    (Rendering|Material|SetVectorParameterValue _returnvalue "BaseColor" _output_get_2 :!class /Script/Engine.MaterialInstanceDynamic)
    (Utilities|Array|Add (Variables|Default|GetCoddingColors) (LocalVariables|GetPickedColor))
    (Utilities|Array|RemoveItem (Variables|Default|GetDifferentColorMeshes) (LocalVariables|GetPickedColor))
    (Default|SetMaterial _array_element _returnvalue)))