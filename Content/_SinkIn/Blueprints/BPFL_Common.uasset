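; Common function library that provides Morse code helpers and a small one-minus math utility.
; ConvertMorseCodeToTimeArray turns a dot-dash string into a timing array: an initial delay, then sign durations separated by gaps.
; Timing values come from small getter functions, with unrecognized signs yielding a negative duration.
; GetNumberFromMorseCode linearly searches a supplied dictionary for the decrypted value, returning a not-found string on failure.
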(fn OneMinus
  (params (Value :type Float%20%28double-precision%29))
  (return (- 1.0 Value)))

(fn ConvertMorseCodetoTimeArray
  (params (MorseCode :type String))
  (bind _timearray (LocalVariables|GetTimeArray))
  (Utilities|Array|Add (LocalVariables|GetTimeArray) (CallFunction|GetInitialDelay))
  (for _array_element (Utilities|String|GetCharacterArrayfromString MorseCode)
    (Utilities|Array|Add (LocalVariables|GetTimeArray) (CallFunction|GetMorseSignTime _array_element))
    (Utilities|Array|Add (LocalVariables|GetTimeArray) (CallFunction|GetDelayTime)))
  (Utilities|Array|RemoveIndex _timearray (- (Utilities|Array|Length _timearray) 1))
  (return (LocalVariables|GetTimeArray)))

(fn GetDotTime
  (return (LocalVariables|GetTime)))

(fn GetDashTime
  (return (LocalVariables|GetTime)))

(fn GetMorseSignTime
  (params (Sign :type String))
  (Utilities|FlowControl|Sequence
    (:then_0
      (if (Utilities|Enum|Equal(Enum) Sign ".")
        (bind _time1 (CallFunction|GetDotTime))
        (return _time1)))
    (:then_1
      (if (Utilities|Enum|Equal(Enum) Sign "-")
        (bind _newparam (CallFunction|GetDashTime))
        (return _newparam)))
    (:then_2
      (return -1.0))))

(fn GetDelayTime
  (return 0.7))

(fn GetInitialDelay
  (return 2.0))

(fn GetNumberfromMorseCode
  (params (Code :type String) (Dictionary :type Morse%20Code%20Dictionary%20Object%20Reference))
  (for _array_element (Variables|/Script/SinkIn.MorseCodeDictionary|GetAvailableMorseCodes Dictionary)
    (if (Utilities|Enum|Equal(Enum) (.MorseCode (Utilities|Struct|BreakDictionaryEntry _array_element)) Code)
      (return (.DecryptedValue (Utilities|Struct|BreakDictionaryEntry _array_element)))))
  (return "Cant find"))