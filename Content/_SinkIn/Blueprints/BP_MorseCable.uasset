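; BP_MorseCable is an interactable spline cable that carries a Morse code the player can hear by connecting a Morse speaker.
; On BeginPlay it moves its sphere to the first or last spline point and picks a random code from the Morse dictionary.
; Interact toggles the connection: it hides the player's speaker and spawns an attached, spline-oriented copy playing the code, or destroys that copy and shows the player's speaker again.
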(event EventBeginPlay
  (if (Variables|Default|GetUseLast)
    (Variables|Default|SetSplineConnectPoint (Spline|GetLocationatSplinePoint (Variables|Default|GetSpline) (- (Spline|GetNumberOfSplinePoints (Variables|Default|GetSpline)) 1) "World"))
    (else
      (bind _output_get (Variables|Default|SetSplineConnectPoint (Spline|GetLocationatSplinePoint (Variables|Default|GetSpline) 0 "World")))))
  (Transformation|SetWorldLocation (Variables|Default|GetSphere) _output_get false false)
  (CallFunction|GetRandomMorseCode))

(event EventInteract
  (params (Player :type BP%20Third%20Person%20Character%20Object%20Reference))
  (bind _bp_morsespeaker (Variables|/Game/ThirdPerson/Blueprints/BP_ThirdPersonCharacter.BP_ThirdPersonCharacter_C|GetBP_MorseSpeaker Player))
  (bind _spline (Variables|Default|GetSpline))
  (Utilities|IsValid (Variables|Default|GetMorseSpeaker)
    (:Is%20Valid
      (Rendering|SetVisibility (Variables|/Game/ThirdPerson/Blueprints/BP_ThirdPersonCharacter.BP_ThirdPersonCharacter_C|GetBP_MorseSpeaker Player) true true)
      (Actor|DestroyActor (Variables|Default|GetMorseSpeaker)))
    (:Is%20Not%20Valid
      (Rendering|SetVisibility _bp_morsespeaker false false)
      (bind _returnvalue (Game|SpawnActorfromClass (Variables|/Script/Engine.ChildActorComponent|GetChildActorClass _bp_morsespeaker) (Math|Transform|MakeTransform (Variables|/Script/Engine.SceneComponent|GetRelativeLocation (Variables|Default|GetSphere)) (Math|Rotator|CombineRotators (Math|Rotator|MakeRotfromX (Spline|GetTangentatDistanceAlongSpline _spline (Variables|/Script/Engine.PrimitiveComponent|GetCachedMaxDrawDistance _spline) "World")) (Math|Rotator|MakeRotator 0.0 0.0 -9e+01)) (Transformation|GetWorldScale _bp_morsespeaker)) "Undefined" "MultiplyWithRoot" 0 0))
      (bind _asbp_morse_speaker (Utilities|Casting|CastToBP_MorseSpeaker _returnvalue))
      (bind _output_get (Variables|Default|SetMorseSpeaker _asbp_morse_speaker))
      (Transformation|AttachActorToActor _output_get self "None" "KeepRelative" "KeepRelative" "KeepWorld" true)
      (Default|Play (Variables|Default|GetMorseSpeaker) (Variables|Default|GetRelatedMorseCode)))))

(fn ConstructionScript)

(fn GetRandomMorseCode
  (Variables|Default|SetRelatedMorseCode (.MorseCode (Utilities|Struct|BreakDictionaryEntry (.OutItem (Utilities|Array|Random (Variables|/Script/SinkIn.MorseCodeDictionary|GetAvailableMorseCodes (Variables|Default|GetMorseCodeDictionary))))))))