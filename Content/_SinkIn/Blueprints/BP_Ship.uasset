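; BP_Ship is a boat that players board and leave by interacting, carrying a diving bell that can be raised and lowered.
; The construction script snaps it to the WaterBodyOcean surface.
; Boarding attaches the player to the Player socket, disables their collision and movement, and adds IMC_Boat input; leaving reverses this.
; MoveBell limits bell travel between its starting height and a line-trace hit below.
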(event EventBeginPlay
  (Variables|Bell|SetBellMaxPos (.Z (Math|Vector|BreakVector (Variables|/Script/Engine.SceneComponent|GetRelativeLocation (Variables|Default|GetBP_DivingBell))))))

(event EventInteract
  (params (Player :type BP%20Third%20Person%20Character%20Object%20Reference))
  (CallFunction|OnInteract Player))

(fn ConstructionScript
  (bind _returnvalue (Actor|GetActorOfClass "/Script/Water.WaterBodyOcean"))
  (Variables|Default|SetWaterBody (Variables|/Script/Water.WaterBody|GetWaterBodyComponent _returnvalue))
  (Transformation|SetActorLocation (.OutWaterSurfaceLocation (CallFunction|GetWaterInfo)) false false))

(fn Possess
  (Pawn|Possess (Game|GetPlayerController 0) self))

(fn GetWaterInfo
  (bind _returnvalue (Transformation|GetActorLocation))
  (bind _waterbody (Variables|Default|GetWaterBody))
  (bind (_outwatersurfacelocation _outwatersurfacenormal _outwatervelocity _outwaterdepth) (WaterBody|GetWaterSurfaceInfoatLocation _waterbody _returnvalue false))
  (return _outwatersurfacelocation _outwatersurfacenormal _outwatervelocity _outwaterdepth))

(fn MoveBell
  (params (Direction :type Float%20%28double-precision%29))
  (bind _bp_divingbell (Variables|Default|GetBP_DivingBell))
  (bind _bellmovespeed (Variables|Bell|GetBellMoveSpeed))
  (bind _returnvalue (Math|Vector|GetUpVector _bp_divingbell))
  (bind _relativelocation (Variables|/Script/Engine.SceneComponent|GetRelativeLocation _bp_divingbell))
  (bind _returnvalue_2 (* _returnvalue Direction))
  (bind _returnvalue_3 (* _returnvalue_2 _bellmovespeed))
  (bind _returnvalue_4 (+ _relativelocation _returnvalue_3))
  (bind _z (Math|Vector|BreakVector _returnvalue_4))
  (if (not (<= _z (.Z (Math|Vector|BreakVector (CallFunction|GetBellMinPos)))))
    (if (not (>= _z (Variables|Bell|GetBellMaxPos)))
      (Transformation|SetRelativeLocation _bp_divingbell _returnvalue_4 false false))))

(fn GetBellMinPos
  (bind _outhit (Collision|LineTraceByChannel (Transformation|GetWorldLocation (Variables|Default|GetBP_DivingBell)) "0.000000,0.000000,-1000.000000" "TraceTypeQuery1" false 0 "None"))
  (return (.Location (Collision|BreakHitResult _outhit))))

(fn OnInteract
  (params (Player :type BP%20Third%20Person%20Character%20Object%20Reference))
  (Variables|/Game/ThirdPerson/Blueprints/BP_ThirdPersonCharacter.BP_ThirdPersonCharacter_C|SetBoat Player self)
  (if (Variables|/Game/ThirdPerson/Blueprints/BP_ThirdPersonCharacter.BP_ThirdPersonCharacter_C|GetIsInBoat Player)
    (Transformation|DetachFromActor Player "KeepWorld" "KeepWorld" "KeepWorld")
    (Transformation|AddRelativeLocation (Variables|Transformation|GetRootComponent) "0.000000,0.000000,60.000000" false false)
    (Collision|SetActorEnableCollision Player true)
    (Pawn|Components|CharacterMovement|SetMovementMode (Variables|/Script/Engine.Character|GetCharacterMovement Player) "MOVE_Walking" 0)
    (Input|RemoveMappingContext (PlayerController|LocalPlayerSubsystems|GetEnhancedInputLocalPlayerSubsystem (Pawn|GetLocalViewingPlayerController Player)) "/Game/_SinkIn/Input/IMC_Boat.IMC_Boat" "(bIgnoreAllPressedKeysUntilRelease=True,bForceImmediately=False,bNotifyUserSettings=False)")
    (Variables|/Game/ThirdPerson/Blueprints/BP_ThirdPersonCharacter.BP_ThirdPersonCharacter_C|SetIsInBoat Player false)
    (Variables|/Game/ThirdPerson/Blueprints/BP_ThirdPersonCharacter.BP_ThirdPersonCharacter_C|SetBoat Player 0)
    (else
      (Pawn|Components|CharacterMovement|SetMovementMode (Variables|/Script/Engine.Character|GetCharacterMovement Player) "MOVE_Walking" 0)
      (Transformation|AttachActorToActor Player self "Player" "SnapToTarget" "SnapToTarget" "KeepWorld" true)
      (Collision|SetActorEnableCollision Player false)
      (Pawn|Components|CharacterMovement|DisableMovement (Variables|/Script/Engine.Character|GetCharacterMovement Player))
      (Input|AddMappingContext (PlayerController|LocalPlayerSubsystems|GetEnhancedInputLocalPlayerSubsystem (Pawn|GetLocalViewingPlayerController Player)) "/Game/_SinkIn/Input/IMC_Boat.IMC_Boat" 1 "(bIgnoreAllPressedKeysUntilRelease=True,bForceImmediately=False,bNotifyUserSettings=False)")
      (Variables|/Game/ThirdPerson/Blueprints/BP_ThirdPersonCharacter.BP_ThirdPersonCharacter_C|SetIsInBoat Player true))))